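; BP_Door is a level exit that shows the win screen once its button has been pressed.
; ButtonPressed calls the Multicast event, which turns the Signal green, sets IfButtonPressed and prints a debug string.
; When a BP_FirstPersonCharacter begins overlapping the Box while that flag is set, the door creates a WP_Win widget and adds it to the viewport.
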(event `self.Box.OnComponentBeginOverlap`
  (params (OverlappedComponent :type "PrimitiveComponent Object Reference") (OtherActor :type "Actor Object Reference") (OtherComp :type "PrimitiveComponent Object Reference") (OtherBodyIndex :type Integer) (bFromSweep :type Boolean) (SweepResult :type "HitResult Structure (by ref)"))
  (cast `/Game/FirstPerson/Blueprints/BP_FirstPersonCharacter` OtherActor)
  (if (`self.ifButtonPressed`)
    (bind _returnvalue (`|CreateWidget` "/Game/blueprints/WP_Win.WP_Win_C"))
    (`UserWidget.AddToViewport` _returnvalue 0)))

(event `ButtonPressed`
  (`self.Multicast`))

(event `Multicast`
  (`PrimitiveComponent.SetMaterial` (`self.Signal`) 0 "/Game/Materials/M_Green.M_Green")
  (set `self.ifButtonPressed` true)
  (`KismetSystemLibrary.PrintString` "William est nul"))

(fn `UserConstructionScript`)