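; BP_PlatformButton is a pressure button that switches its linked Platforms between pressed and not-pressed behavior.
; Box overlap begin and end drive separate timelines that move the Mesh on Z.
; Pressing calls WhileButtonPressed on BP_JumpPlatform entries once the down animation finishes and sets IsActivated, which is never cleared here.
; Release calls WhileButtonIsNotPressed immediately, without waiting for the up animation.
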(event `self.Box.OnComponentBeginOverlap`
  (params (OverlappedComponent :type "PrimitiveComponent Object Reference") (OtherActor :type "Actor Object Reference") (OtherComp :type "PrimitiveComponent Object Reference") (OtherBodyIndex :type Integer) (bFromSweep :type Boolean) (SweepResult :type "HitResult Structure (by ref)"))
  (bind _mesh (`self.Mesh`))
  (bind (_relativelocation_x _relativelocation_y) (`KismetMathLibrary.BreakVector` (`SceneComponent.RelativeLocation` _mesh)))
  (bind (_direction _newtrack_0) (`Timeline|ButtonDown`)
    (:`Update`
      (`SceneComponent.K2_SetRelativeLocation` _mesh (`KismetMathLibrary.MakeVector` _relativelocation_x _relativelocation_y _newtrack_0) false false))
    (:`Finished`
      (for _array_element (`self.Platforms`)
        (bind _asbp_jump_platform (cast `/Game/blueprints/BP_JumpPlatform` _array_element))
        (`/Game/blueprints/BP_JumpPlatform.whileButtonPressed` _asbp_jump_platform)
        (set `self.bIsActivated` true)))))

(event `self.Box.OnComponentEndOverlap`
  (params (OverlappedComponent :type "PrimitiveComponent Object Reference") (OtherActor :type "Actor Object Reference") (OtherComp :type "PrimitiveComponent Object Reference") (OtherBodyIndex :type Integer))
  (bind _mesh (`self.Mesh`))
  (bind (_relativelocation_x _relativelocation_y) (`KismetMathLibrary.BreakVector` (`SceneComponent.RelativeLocation` _mesh)))
  (`|ExecutionSequence`
    (:`then_0`
      (bind (_direction _buttonup) (`Timeline|ButtonUp`)
        (:`Update`
          (`SceneComponent.K2_SetRelativeLocation` _mesh (`KismetMathLibrary.MakeVector` _relativelocation_x _relativelocation_y _buttonup) false false))))
    (:`then_1`
      (for _array_element (`self.Platforms`)
        (`/Game/blueprints/BP_JumpPlatform.whileButtonIsNotPressed` _array_element)))))

(fn `UserConstructionScript`)